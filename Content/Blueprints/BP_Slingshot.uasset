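; BP_Slingshot is a pinball slingshot that kicks away any overlapping Ball and awards points through PinballGameMode.
; The kick is a velocity-change impulse along the capsule's forward vector, so it ignores the ball's mass.
; Each hit restarts a timeline that drives the PercentOut parameter on a dynamic material, created in the construction script for one mesh slot, to animate the bounce.
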(event EventBeginPlay)

(event Collision|EventActorBeginOverlap
  (params (OtherActor :type Actor%20Object%20Reference))
  (bind _asball (Utilities|Casting|CastToBall OtherActor))
  (bind _aspinball_game_mode (Utilities|Casting|CastToPinballGameMode (Game|GetGameMode)))
  (Default|AddScore _aspinball_game_mode 2e+01)
  (Physics|AddImpulse (Variables|/Game/Blueprints/Ball.Ball_C|GetBall _asball) (* (Math|Vector|GetForwardVector (Variables|Default|GetCapsule)) 2.5e+03) "None" true)
  (bind _bounce (Timeline|Timeline_0 PlayFromStart)
    (:Update
      (bind _asmaterial_instance_dynamic (Utilities|Casting|CastToMaterialInstanceDynamic (Rendering|Material|GetMaterial (Variables|Default|GetStaticMesh) 2)))
      (Rendering|Material|SetScalarParameterValue _asmaterial_instance_dynamic "PercentOut" _bounce :!class /Script/Engine.MaterialInstanceDynamic))))

(event EventTick
  (params (DeltaSeconds :type Float%20%28single-precision%29)))

(fn ConstructionScript
  (Rendering|Material|CreateDynamicMaterialInstance (Variables|Default|GetStaticMesh) 2 0 :!class /Script/Engine.PrimitiveComponent))