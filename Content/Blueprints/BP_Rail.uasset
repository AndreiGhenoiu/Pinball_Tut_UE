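; BP_Rail is a rail actor that builds its visible mesh along an editable spline.
; The construction script adds a spline mesh component for each segment, matching positions and tangents to the spline points in local space.
; The first segment uses a start mesh with an adjustable X start scale, the last an end mesh, and those between a middle mesh.
; It has no runtime logic.
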(event EventBeginPlay)

(event Collision|EventActorBeginOverlap
  (params (OtherActor :type Actor%20Object%20Reference)))

(event EventTick
  (params (DeltaSeconds :type Float%20%28single-precision%29)))

(fn ConstructionScript
  (bind _spline (Variables|Default|GetSpline))
  (bind _spline_2 (Variables|Default|GetSpline))
  (bind _returnvalue (Spline|GetNumberOfSplinePoints _spline_2))
  (bind _returnvalue_2 (- _returnvalue 2))
  (for _index (range 0 _returnvalue_2)
    (bind _returnvalue_3 (AddComponent|AddSplineMeshComponent false))
    (if (== _index 0)
      (Components|StaticMesh|SetStaticMesh _returnvalue_3 (Variables|Default|GetRailStartMesh))
      (SplineMesh|SetStartScale _returnvalue_3 (Math|Vector2D|MakeVector2D (Variables|Default|GetInitialScale) 1.0) true :!class /Script/Engine.SplineMeshComponent)
      (elif (== _index _returnvalue_2)
        (Components|StaticMesh|SetStaticMesh _returnvalue_3 (Variables|Default|GetRailEndMesh))
        (else
          (Components|StaticMesh|SetStaticMesh _returnvalue_3 (Variables|Default|GetRailMidMesh)))))
    (SplineMesh|SetStartandEnd _returnvalue_3 (.Location (Spline|GetLocationandTangentatSplinePoint _spline _index "Local")) (.Tangent (Spline|GetLocationandTangentatSplinePoint _spline _index "Local")) (.Location (Spline|GetLocationandTangentatSplinePoint _spline (+ _index 1) "Local")) (.Tangent (Spline|GetLocationandTangentatSplinePoint _spline (+ _index 1) "Local")) true :!class /Script/Engine.SplineMeshComponent)))