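; Flipper actor, likely pinball-style, that swings a Flipper component between a rest angle and an opposite end angle.
; The construction script picks the angles from FlipType (Left or Right), applies the rest rotation and mirrors the component with negative X scale for Right.
; Flip and Flop events use MoveComponentTo to rotate to the end and back over FlipTime.
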(event Custom|Flop
  (Components|MoveComponentTo (Variables|Default|GetFlipper) "0, 0, 0" (Variables|Default|GetstartRotation) false false (Variables|Default|GetflipTime) false))

(event Custom|Flip
  (Components|MoveComponentTo (Variables|Default|GetFlipper) "0, 0, 0" (Variables|Default|GetendRotation) false false (Variables|Default|GetflipTime) false))

(event EventBeginPlay)

(event Collision|EventActorBeginOverlap
  (params (OtherActor :type Actor%20Object%20Reference)))

(event EventTick
  (params (DeltaSeconds :type Float%20%28single-precision%29)))

(fn ConstructionScript
  (bind _fliptype (Variables|Default|GetflipType))
  (bind _returnvalue (Utilities|Select :Index _fliptype :NewEnumerator0 "0,20.000000, 0" :NewEnumerator1 "0.000000,-20.000000,0.000000"))
  (Variables|Default|SetstartRotation _returnvalue)
  (Variables|Default|SetendRotation (* _returnvalue -1))
  (Transformation|SetRelativeRotation (Variables|Default|GetFlipper) (Variables|Default|GetstartRotation) false false)
  (switch Utilities|FlowControl|Switch|SwitchonflipType (Variables|Default|GetflipType)
    (:NewEnumerator1
      (Transformation|SetRelativeScale3D (Variables|Default|GetFlipper) "-1.000000,1.000000,1.000000"))))