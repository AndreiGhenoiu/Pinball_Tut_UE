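; Player controller for a pinball game that routes input to the table's flippers and plunger and shows the HUD.
; On BeginPlay it gathers Flipper actors into left and right lists by FlipType, caches the first plunger found, and creates the PinballHUD widget.
; Left and right flipper inputs call Flip on press and Flop on release for every flipper on that side.
; The plunger input starts charging on press and stops on release.
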(event Custom|detectFlippers
  (bind _outactors (Actor|GetAllActorsOfClass "/Game/Blueprints/flipper.flipper_C"))
  (for _array_element _outactors
    (switch Utilities|FlowControl|Switch|SwitchonflipType (Variables|/Game/Blueprints/flipper.flipper_C|GetflipType _array_element)
      (:NewEnumerator0
        (Utilities|Array|Add (Variables|Default|GetleftFlippers) _array_element))
      (:NewEnumerator1
        (Utilities|Array|Add (Variables|Default|GetrightFlippers) _array_element)))))

(event Custom|CreatePlayerHUD
  (Viewport|RemoveAllWidgets)
  (bind _returnvalue (UserInterface|CreateWidget "/Game/Blueprints/PinballHUD.PinballHUD_C"))
  (UserInterface|Viewport|AddtoViewport _returnvalue 0))

(event Custom|detectPlunger
  (bind _outactors (Actor|GetAllActorsOfClass "/Game/Blueprints/BP_PLUNGER.BP_PLUNGER_C"))
  (Variables|Default|Setplunger (Utilities|Array|Get(acopy) _outactors)))

(event EventBeginPlay
  (CallFunction|DetectFlippers)
  (CallFunction|DetectPlunger)
  (CallFunction|CreatePlayerHUD))

(event EventTick
  (params (DeltaSeconds :type Float%20%28single-precision%29)))

(event Input|ActionEvents|InputActionLeft_Flipper
  (params (Key :type Key%20Structure))
  (bind _leftflippers (Variables|Default|GetleftFlippers))
  (:Pressed
    (for _array_element _leftflippers
      (Default|Flip _array_element)))
  (:Released
    (for _array_element_2 _leftflippers
      (Default|Flop _array_element_2))))

(event Input|ActionEvents|InputActionRight_Flipper
  (params (Key :type Key%20Structure))
  (bind _rightflippers (Variables|Default|GetrightFlippers))
  (:Pressed
    (for _array_element _rightflippers
      (Default|Flip _array_element)))
  (:Released
    (for _array_element_2 _rightflippers
      (Default|Flop _array_element_2))))

(event Input|ActionEvents|InputActionplunger
  (params (Key :type Key%20Structure))
  (bind _plunger (Variables|Default|Getplunger))
  (:Pressed
    (Default|ChargePlunger _plunger))
  (:Released
    (Default|StopCharge _plunger)))

(fn ConstructionScript)